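; AI controller for guard enemies that runs the BT_Guard behavior tree and feeds it perception results through the Blackboard.
; On each perception update, it switches on the stimulus tag.
; Hearing stimuli store the noise location in the Blackboard.
; Any other stimulus stores the player character as the target reference, without checking the sensed actor or whether sensing succeeded.
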(event `self.ReceiveBeginPlay`
  (`self.RunBehaviorTree` "/Game/Blueprints/Enemy/BT_Guard.BT_Guard"))

(event `self.AIPerception.OnTargetPerceptionUpdated`
  (params (Actor :type "Actor Object Reference") (Stimulus :type "AIStimulus Structure"))
  (bind (_age _expirationage _strength _stimuluslocation _receiverlocation _tag) (break `AIStimulus` Stimulus))
  (switch `name` _tag
    (:`Default`
      (`BlackboardComponent.SetValueAsObject` (`self.Blackboard`) (`self.playerRefKey`) (`GameplayStatics.GetPlayerCharacter` 0)))
    (:`Hearing`
      (bind _output_get (set `self.Hearing Stimulus Location` _stimuluslocation))
      (`BlackboardComponent.SetValueAsVector` (`self.Blackboard`) (`self.hearing Location Ref Key`) _output_get))))

(fn `UserConstructionScript`)