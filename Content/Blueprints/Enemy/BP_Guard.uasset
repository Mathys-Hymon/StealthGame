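; BP_Guard is an enemy guard Blueprint that can return to its starting position when the game resets.
; BeginPlay calls the parent and caches the actor's location, which the ResetGame event restores without sweeping.
; Only location is restored, and the file adds no other behavior beyond calls to parent logic.
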(event `self.ReceiveBeginPlay`
  (`parent.ReceiveBeginPlay`)
  (set `self.initialLocation` (`self.K2_GetActorLocation`)))

(event `/Game/Blueprints/BPI/BPI_Enemy.ResetGame`
  (`self.K2_SetActorLocation` (`self.initialLocation`)))

(fn `UserConstructionScript`
  (`parent.UserConstructionScript`))