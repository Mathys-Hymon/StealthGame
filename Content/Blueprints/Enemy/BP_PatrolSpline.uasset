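; BP_PatrolSpline is an enemy patrol path that moves a BP_PatrolTarget along a spline as the point to follow.
; BeginPlay spawns the target at the first spline point, and StartPatrol and StopPatrol play and stop a Timeline that lerps it along the spline's distance.
; The play rate scales inversely with spline length, keeping travel speed consistent across paths of different lengths.
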(event `self.ReceiveBeginPlay`
  ;[1 1 1] Create the target, which the player will follow
  (bind _returnvalue (`|SpawnActorFromClass` "/Game/Blueprints/Enemy/BP_PatrolTarget.BP_PatrolTarget_C" (`KismetMathLibrary.Conv_VectorToTransform` (`SplineComponent.GetLocationAtSplinePoint` (`self.Spline`) 0 "World")) "Undefined" "MultiplyWithRoot" null null))
  (set `self.sphere` _returnvalue))

(event `StartPatrol`
  ;[1 1 1] Move the target along the spline
  (`TimelineComponent.SetPlayRate` (`self.Timeline`) (/ 1.0 (/ (`SplineComponent.GetSplineLength` (`self.Spline`)) 300.0)))
  (bind (_direction _alpha) (`Timeline|Timeline` :!label _label)
    (:`Update`
      (`self.K2_SetActorLocation` (`self.sphere`) (`SplineComponent.GetLocationAtDistanceAlongSpline` (`self.Spline`) (`KismetMathLibrary.Lerp` 0.0 (`SplineComponent.GetDistanceAlongSplineAtSplinePoint` (`self.Spline`) (`SplineComponent.GetNumberOfSplinePoints` (`self.Spline`))) _alpha) "World") false false))))

(event `StopPatrol`
  ;[1 1 1] Move the target along the spline
  (goto _label :!via `Stop`))

(fn `UserConstructionScript`)