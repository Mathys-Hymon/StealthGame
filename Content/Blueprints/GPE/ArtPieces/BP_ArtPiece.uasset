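; BP_ArtPiece is an interactable art piece that grants a score and reports itself as a masterpiece when taken.
; While its mesh is visible, the widget trigger sends its pattern to the player HUD as a password message.
; Interacting hides the mesh and interaction widget, shows the optional idle Niagara effect, fires a coin burst and returns the score with the masterpiece flag.
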(event `/Game/Blueprints/BPI/BPI_Interaction.TriggerWidget`
  (if (`SceneComponent.IsVisible` (`self.SM_Art`))
    (message `/Game/Blueprints/BPI/BPI_HUD.Password` (`PlayerController.GetHUD` (`GameplayStatics.GetPlayerController` 0)) (`self.Patern`))))

(fn `Interact`
  (returns (score :type Integer) (isMasterPiece :type Boolean))
  (bind _idlefx (`self.idleFX`))
  (`SceneComponent.SetVisibility` (`self.SM_Art`) false false)
  (`SceneComponent.SetVisibility` (`self.W_Interaction`) false false)
  (`/Engine/EditorBlueprintResources/StandardMacros.IsValid` _idlefx
    (:`Is Valid`
      (`SceneComponent.SetVisibility` (`NiagaraActor.NiagaraComponent` _idlefx) true false))
    (:`Is Not Valid`
      _))
  (`ActorComponent.Activate` (`self.NS_CoinBurst2`) false)
  (return (`self.score`) true))

(fn `UserConstructionScript`
  (`parent.UserConstructionScript`))