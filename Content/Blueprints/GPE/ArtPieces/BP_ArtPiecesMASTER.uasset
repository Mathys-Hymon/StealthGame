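; Master Blueprint for art piece interactables, with a configurable mesh applied in the construction script.
; ShowInteraction toggles the prompt widget and pickup Niagara effect, showing them only while the art mesh is visible; both start hidden.
; Reset makes the mesh visible again, along with the idle effect if one is assigned.
; Interact returns default zero score and non-masterpiece values, and InteractorType reports the piece's interactor category.
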(event `/Game/Blueprints/BPI/BPI_Interaction.ShowInteraction`
  (params (show :type Boolean))
  (bind _returnvalue (and show (`SceneComponent.IsVisible` (`self.SM_Art`))))
  (`SceneComponent.SetVisibility` (`self.W_Interaction`) _returnvalue false)
  (`SceneComponent.SetVisibility` (`self.NS_Pickup_4`) _returnvalue false))

(event `self.ReceiveBeginPlay`
  (`SceneComponent.SetVisibility` (`self.W_Interaction`) false false)
  (`SceneComponent.SetVisibility` (`self.NS_Pickup_4`) false false))

(event `/Game/Blueprints/BPI/BPI_Interaction.Reset`
  (bind _idlefx (`self.idleFX`))
  (`SceneComponent.SetVisibility` (`self.SM_Art`) true false)
  (`/Engine/EditorBlueprintResources/StandardMacros.IsValid` _idlefx
    (:`Is Valid`
      (`SceneComponent.SetVisibility` (`NiagaraActor.NiagaraComponent` _idlefx) true false))))

(fn `Interact`
  (returns (score :type Integer) (isMasterPiece :type Boolean))
  (return 0 false))

(fn `InteractorType`
  (returns (type :type "/Game/Blueprints/BPI/Enum_InteractorType Enum"))
  (return "NewEnumerator0"))

(fn `UserConstructionScript`
  (`StaticMeshComponent.SetStaticMesh` (`self.SM_Art`) (`self.mesh`)))