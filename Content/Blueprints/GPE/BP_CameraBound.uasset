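; BP_CameraBound is a trigger volume that moves the player camera when a player enters it.
; In the editor, its construction script places a preview camera from CamLoc plus the data asset's camera offset, half standing capsule height and rotation.
; On BeginPlay it caches that camera's world location and destroys the component.
; Overlapping BPI_Player actors receive MoveCameraMessage with the cached location and a lerp speed.
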(event `self.ReceiveBeginPlay`
  (set `self.targetLoc` (`SceneComponent.K2_GetComponentLocation` (`self.previewCamera`)))
  (`ActorComponent.K2_DestroyComponent` (`self.previewCamera`)))

(event `self.DetectionBox.OnComponentBeginOverlap`
  (params (OverlappedComponent :type "PrimitiveComponent Object Reference") (OtherActor :type "Actor Object Reference") (OtherComp :type "PrimitiveComponent Object Reference") (OtherBodyIndex :type Integer) (bFromSweep :type Boolean) (SweepResult :type "HitResult Structure (by ref)"))
  (if (`KismetSystemLibrary.DoesImplementInterface` OtherActor "/Game/Blueprints/BPI/BPI_Player.BPI_Player_C")
    (message `/Game/Blueprints/BPI/BPI_Player.MoveCamera` OtherActor (`self.targetLoc`) (`self.lerpSpeed`))))

(fn `UserConstructionScript`
  (bind _dataassetref (`self.dataAssetRef`))
  (set `self.targetLoc` (`SceneComponent.K2_GetComponentLocation` (`self.previewCamera`)))
  (`SceneComponent.K2_SetRelativeLocation` (`self.previewCamera`) (+ (`self.camLoc`) (`/Game/DataAsset/BP_DataAsset.cameraOffset` _dataassetref) (`KismetMathLibrary.MakeVector` 0.0 0.0 (/ (`/Game/DataAsset/BP_DataAsset.standingCapsuleSize` _dataassetref) 2.0))) false false)
  (`SceneComponent.K2_SetRelativeRotation` (`self.previewCamera`) (`/Game/DataAsset/BP_DataAsset.cameraRotation` _dataassetref) false false))