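; Level exit door for the stealth game that moves the player on to the next area or ends the game.
; Its interaction prompt and lockpick HUD widget respond only when the player holds the master piece.
; Interacting teleports the player to NextSpawnPoint, updates their spawn position, and resets level score and master-piece state.
; Without a valid spawn point, it shows the end-game widget and plays its score bounce animation.
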(event `self.ReceiveBeginPlay`
  (`SceneComponent.SetVisibility` (`self.W_Interaction`) false false))

(event `/Game/Blueprints/BPI/BPI_Interaction.TriggerWidget`
  (bind _masterpiece (message `/Game/Blueprints/BPI/BPI_Player.HasMasterPiece` (`GameplayStatics.GetPlayerCharacter` 0)))
  (if _masterpiece
    (message `/Game/Blueprints/BPI/BPI_HUD.Lockpick` (`PlayerController.GetHUD` (`GameplayStatics.GetPlayerController` 0)) (`self.Widget`))))

(event `/Game/Blueprints/BPI/BPI_Interaction.ShowInteraction`
  (params (show :type Boolean))
  (bind _masterpiece (message `/Game/Blueprints/BPI/BPI_Player.HasMasterPiece` (`GameplayStatics.GetPlayerCharacter` 0)))
  (if _masterpiece
    (`SceneComponent.SetVisibility` (`self.W_Interaction`) show false)))

(fn `Interact`
  (returns (score :type Integer) (isMasterPiece :type Boolean))
  (bind _returnvalue (`GameplayStatics.GetPlayerCharacter` 0))
  (bind _returnvalue_2 (`self.K2_GetActorLocation` (`self.nextSpawnPoint`)))
  (bind _returnvalue_3 (`PlayerController.GetHUD` (`GameplayStatics.GetPlayerController` 0)))
  (`/Engine/EditorBlueprintResources/StandardMacros.IsValid` (`self.nextSpawnPoint`)
    (:`Is Valid`
      (`self.K2_SetActorLocation` _returnvalue _returnvalue_2 false false)
      (message `/Game/Blueprints/BPI/BPI_Player.NewSpawnPos` _returnvalue _returnvalue_2)
      (bind _asgi_stealth_game (cast `/Game/_Manager/inGame/GI_StealthGame` (`GameplayStatics.GetGameInstance`)))
      (set `/Game/_Manager/inGame/GI_StealthGame.scoreInLevel` 0 _asgi_stealth_game)
      (message `/Game/Blueprints/BPI/BPI_Player.ResetHasMasterPiece` (`GameplayStatics.GetPlayerCharacter` 0))
      (return 0 false))
    (:`Is Not Valid`
      (message `/Game/Blueprints/BPI/BPI_HUD.AddWidget` _returnvalue_3 "/Game/Blueprints/UI/WB_EndGame.WB_EndGame_C" false)
      (bind _ashud_player (cast `/Game/_Manager/inGame/HUD_Player` _returnvalue_3))
      (bind _endgamewidget (`/Game/_Manager/inGame/HUD_Player.endGameWidget` _ashud_player))
      (`UserWidget.PlayAnimation` _endgamewidget (`/Game/Blueprints/UI/WB_EndGame.BounceScoreEnd` _endgamewidget) 0.0 1 "Forward" 1.0 false))))

(fn `InteractorType`
  (returns (type :type "/Game/Blueprints/BPI/Enum_InteractorType Enum"))
  (return "NewEnumerator1"))

(fn `UserConstructionScript`)