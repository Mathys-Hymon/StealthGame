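; Security camera that sweeps between two yaw limits and alerts enemies when it spots the player.
; A moving player in the detection cone with a clear line trace turns it red, and it rotates to track them.
; Each tick while alerted, it sends the seen location to all BPI_Enemy actors, resetting shortly after cone exit.
; Construction script previews both sweep extremes with extra cones, destroyed at BeginPlay.
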(event `self.ReceiveBeginPlay`
  (bind _detectionsize (`self.detectionSize`))
  (`SceneComponent.SetWorldScale3D` (`self.Cone`) (`KismetMathLibrary.MakeVector` _detectionsize _detectionsize (`self.detectionLength`)))
  (`SceneComponent.K2_SetRelativeRotation` (`self.Camera`) (`KismetMathLibrary.MakeRotator` 0.0 (`self.detectionAngle`)) false false)
  (for _array_element (`|MakeArray` (`self.CameraPreview1`) (`self.Cone1`) (`self.Cone2`) (`self.CameraPreview2`))
    (`ActorComponent.K2_DestroyComponent` _array_element)
    (bind _outactors (`GameplayStatics.GetAllActorsWithInterface` "/Game/Blueprints/BPI/BPI_Enemy.BPI_Enemy_C"))
    (set `self.AllEnemies` _outactors)))

(event `self.ReceiveTick`
  (params (DeltaSeconds :type "Float (single-precision)"))
  (bind _seenactorref (`self.seenActorRef`))
  (bind _camera (`self.Camera`))
  (bind _seenactorref_2 (`self.seenActorRef`))
  (bind _lastseenloc (`self.lastSeenLoc`))
  (bind _returnvalue (`self.K2_GetActorLocation` _seenactorref))
  (bind (_relativerotation_roll _relativerotation_pitch _relativerotation_yaw) (`KismetMathLibrary.BreakRotator` (`SceneComponent.RelativeRotation` _camera)))
  (bind _output (`|GetArrayItem` (`PrimitiveComponent.GetOverlappingActors` (`self.Cone`) "/Game/Blueprints/Player/BP_Player.BP_Player_C")))
  (`|ExecutionSequence`
    (:`then_0`
      (if (not (`self.seePlayer`))
        (if (`KismetMathLibrary.NearlyEqual_FloatFloat` _relativerotation_yaw (`self.maxRotationAngle`) 0.5)
          (set `self.goRight` true)
          (elif (`KismetMathLibrary.NearlyEqual_FloatFloat` _relativerotation_yaw (`self.minRotationAngle`) 0.5)
            (set `self.goRight` false)))
        (`SceneComponent.K2_SetRelativeRotation` _camera (`KismetMathLibrary.MakeRotator` _relativerotation_roll _relativerotation_pitch (`KismetMathLibrary.FInterpTo_Constant` _relativerotation_yaw (`KismetMathLibrary.SelectFloat` (`self.minRotationAngle`) (`self.maxRotationAngle`) (`self.goRight`)) (`GameplayStatics.GetWorldDeltaSeconds`) 50.0)) false false)))
    (:`then_1`
      (if (`self.seePlayer`)
        (`/Engine/EditorBlueprintResources/StandardMacros.IsValid` _seenactorref
          (:`Is Valid`
            (`self.RotateWhenSeen` _returnvalue)
            (for _array_element (`self.AllEnemies`)
              (message `/Game/Blueprints/BPI/BPI_Enemy.SendSeenLocation` _array_element _returnvalue)))
          (:`Is Not Valid`
            (`self.RotateWhenSeen` _lastseenloc)
            (for _array_element_2 (`self.AllEnemies`)
              (message `/Game/Blueprints/BPI/BPI_Enemy.SendSeenLocation` _array_element_2 _lastseenloc))))))
    (:`then_2`
      (`/Engine/EditorBlueprintResources/StandardMacros.IsValid` _output
        (:`Is Valid`
          (if (> (`KismetMathLibrary.VSize` (`self.GetVelocity` _output)) 0.0)
            (bind _outhit (`KismetSystemLibrary.LineTraceSingle` (`SceneComponent.K2_GetComponentLocation` (`self.Camera`)) (`self.K2_GetActorLocation` _output) "TraceTypeQuery1"))
            (bind (_bblockinghit _binitialoverlap _time _distance _location _impactpoint _normal _impactnormal _physmat _hitactor) (`GameplayStatics.BreakHitResult` _outhit))
            (if (`KismetSystemLibrary.DoesImplementInterface` _hitactor "/Game/Blueprints/BPI/BPI_Player.BPI_Player_C")
              (set `self.seenActorRef` _hitactor)
              (set `self.seePlayer` true)
              (`PrimitiveComponent.SetMaterial` (`self.Camera`) 0 "/AnimationSharing/AnimSharingRed.AnimSharingRed")
              (else
                (if (`KismetSystemLibrary.IsValid` _seenactorref_2)
                  (set `self.lastSeenLoc` (`self.K2_GetActorLocation` _seenactorref_2)))
                (set `self.seenActorRef` null)
                (set `self.seePlayer` false)
                (`PrimitiveComponent.SetMaterial` (`self.Camera`) 0 "/Engine/BasicShapes/BasicShapeMaterial.BasicShapeMaterial")))))))))

(event `self.Cone.OnComponentEndOverlap`
  (params (OverlappedComponent :type "PrimitiveComponent Object Reference") (OtherActor :type "Actor Object Reference") (OtherComp :type "PrimitiveComponent Object Reference") (OtherBodyIndex :type Integer))
  (if (`KismetSystemLibrary.DoesImplementInterface` OtherActor "/Game/Blueprints/BPI/BPI_Player.BPI_Player_C")
    (set `self.lastSeenLoc` (`self.K2_GetActorLocation` OtherActor))
    (set `self.seenActorRef` null)
    (`KismetSystemLibrary.RetriggerableDelay` 2.0)
    (set `self.lastSeenLoc` (0.0 0.0 0.0))
    (set `self.seePlayer` false)
    (`PrimitiveComponent.SetMaterial` (`self.Camera`) 0 "/Engine/BasicShapes/BasicShapeMaterial.BasicShapeMaterial")))

(fn `RotateWhenSeen`
  (params (Start :type "Vector Structure (by ref)"))
  (bind _camera (`self.Camera`))
  (bind (_relativerotation_roll _relativerotation_pitch _relativerotation_yaw) (`KismetMathLibrary.BreakRotator` (`SceneComponent.RelativeRotation` _camera)))
  (bind (_returnvalue_roll _returnvalue_pitch _returnvalue_yaw) (`KismetMathLibrary.BreakRotator` (`KismetMathLibrary.FindLookAtRotation` Start (`SceneComponent.K2_GetComponentLocation` (`self.Camera`)))))
  (`SceneComponent.K2_SetRelativeRotation` _camera (`KismetMathLibrary.MakeRotator` _relativerotation_roll _relativerotation_pitch (`KismetMathLibrary.FClamp` (`KismetMathLibrary.FInterpTo_Constant` _relativerotation_yaw _returnvalue_yaw (`GameplayStatics.GetWorldDeltaSeconds`) 30.0) -45.0 45.0)) false false)
  (return))

(fn `UserConstructionScript`
  (bind _detectionsize (`self.detectionSize`))
  (bind _detectionsize_2 (`self.detectionSize`))
  (bind _detectionsize_3 (`self.detectionSize`))
  (`|ExecutionSequence`
    (:`then_0`
      (`SceneComponent.SetWorldScale3D` (`self.Cone`) (`KismetMathLibrary.MakeVector` _detectionsize_3 _detectionsize_3 (`self.detectionLength`)))
      (`SceneComponent.K2_SetRelativeRotation` (`self.Camera`) (`KismetMathLibrary.MakeRotator` 0.0 (`self.detectionAngle`)) false false))
    (:`then_1`
      (`SceneComponent.SetWorldScale3D` (`self.Cone1`) (`KismetMathLibrary.MakeVector` _detectionsize_2 _detectionsize_2 (`self.detectionLength`)))
      (`SceneComponent.K2_SetRelativeRotation` (`self.CameraPreview1`) (`KismetMathLibrary.MakeRotator` 0.0 (`self.detectionAngle`) (`self.minRotationAngle`)) false false))
    (:`then_2`
      (`SceneComponent.SetWorldScale3D` (`self.Cone2`) (`KismetMathLibrary.MakeVector` _detectionsize _detectionsize (`self.detectionLength`)))
      (`SceneComponent.K2_SetRelativeRotation` (`self.CameraPreview2`) (`KismetMathLibrary.MakeRotator` 0.0 (`self.detectionAngle`) (`self.maxRotationAngle`)) false false))))