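; Player character for a stealth art-theft game, with camera-relative movement, a timeline-driven crouch and tuning from a data asset.
; A detached spring arm is repositioned by MoveCamera, and looping footstep noise, quieter when crouched, feeds AI hearing.
; Overlapped BPI_Interaction actors can start lockpicking: wins animate score and record masterpieces, losses make noise.
; ResetGame restores art pieces and guards, returns to spawn and removes the level's score.
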(event `self.ReceiveBeginPlay`
  ;[0 0.2542 0.2423] Detach Camera from Player
  (`SceneComponent.K2_DetachFromComponent` (`self.SpringArm`) "KeepWorld" "KeepWorld" "KeepWorld" true)
  (`KismetSystemLibrary.K2_SetTimerDelegate` (delegate `FootstepSound`) 0.5 true)
  (set `CharacterMovementComponent.MaxWalkSpeed` (`/Game/DataAsset/BP_DataAsset.walkSpeed` (`self.dataAssetRef`)) (`self.CharacterMovement`))
  (bind _asgi_stealth_game (cast `/Game/_Manager/inGame/GI_StealthGame` (`GameplayStatics.GetGameInstance`)))
  (set `self.gameInstanceRef` _asgi_stealth_game)
  (set `self.spawnPos` (`self.K2_GetActorLocation`))
  (bind _ashud_player (cast `/Game/_Manager/inGame/HUD_Player` (`PlayerController.GetHUD` (`GameplayStatics.GetPlayerController` 0))))
  (set `self.As HUD Player` _ashud_player))

(event `FootstepSound`
  (bind _dataassetref (`self.dataAssetRef`))
  ;[0 0.3661 0.4635] MakeFootstepsSounds
  (if (> (`self.movementVelocity`) 0.0)
    (`self.MakeNoise` (`KismetMathLibrary.SelectFloat` (`/Game/DataAsset/BP_DataAsset.crouchVolume` _dataassetref) (`/Game/DataAsset/BP_DataAsset.walkVolume` _dataassetref) (`self.isCrouched`)) null (`self.K2_GetActorLocation`) 0.0 "Hearing")))

(event `/Game/Blueprints/BPI/BPI_Player.MoveCamera`
  (params (newPos :type "Vector Structure") (newRot :type "Rotator Structure") (lerpSpeed :type "Float (double-precision)"))
  (bind _springarm (`self.SpringArm`))
  ;[0 0.2542 0.2423] MoveCamera
  (`SceneComponent.K2_SetWorldLocationAndRotation` _springarm newPos newRot false false)
  (set `SpringArmComponent.CameraLagSpeed` lerpSpeed _springarm)
  (set `SpringArmComponent.CameraRotationLagSpeed` lerpSpeed _springarm))

(event `/Game/Blueprints/BPI/BPI_Player.CanMove`
  (params (move :type Boolean))
  (set `self.movementEnable` move))

(event `/Game/Blueprints/BPI/BPI_Player.Move`
  (params (axis :type "Vector2D Structure"))
  (bind (_x _y) (`KismetMathLibrary.BreakVector2D` axis))
  (bind _returnvalue (`PlayerCameraManager.GetCameraRotation` (`GameplayStatics.GetPlayerCameraManager` 0)))
  ;[0 0.2542 0.2423] MovePlayer
  (if (`self.movementEnable`)
    (set `self.movementVelocity` (`KismetMathLibrary.VSize2D` axis))
    (`self.AddMovementInput` (`KismetMathLibrary.GetForwardVector` _returnvalue) _y)
    (`self.AddMovementInput` (`KismetMathLibrary.GetRightVector` _returnvalue) _x)))

(event `/Game/Blueprints/BPI/BPI_Player.CrouchPlayer`
  (bind _dataassetref (`self.dataAssetRef`))
  (bind _charactermovement (`self.CharacterMovement`))
  (bind _dataassetref_2 (`self.dataAssetRef`))
  (bind _crouchcapsulesize (`/Game/DataAsset/BP_DataAsset.crouchCapsuleSize` _dataassetref))
  ;[0 0.2542 0.2423] CrouchPlayer
  (if (not (`self.isCrouched`))
    (set `self.isCrouched` true)
    (set `CharacterMovementComponent.MaxWalkSpeed` (`/Game/DataAsset/BP_DataAsset.crouchSpeed` _dataassetref_2) _charactermovement)
    (bind (_direction _lerp) (`Timeline|CrouchTimeline` :!label _label)
      (:`Update`
        (`CapsuleComponent.SetCapsuleHalfHeight` (`self.CapsuleComponent`) (`KismetMathLibrary.Lerp` (`/Game/DataAsset/BP_DataAsset.standingCapsuleSize` _dataassetref) _crouchcapsulesize _lerp) true)
        (`SceneComponent.K2_SetRelativeLocation` (`self.Mesh`) (`KismetMathLibrary.MakeVector` 0.0 0.0 (`KismetMathLibrary.Lerp` -90.0 (+ -90.0 _crouchcapsulesize) _lerp)) false false)))
    (else
      (set `self.isCrouched` false)
      (set `CharacterMovementComponent.MaxWalkSpeed` (`/Game/DataAsset/BP_DataAsset.walkSpeed` _dataassetref_2) _charactermovement)
      (goto _label :!via `Reverse`))))

(event `/Game/Blueprints/BPI/BPI_Player.Interact`
  (bind _interactableactor (`self.interactableActor`))
  ;[0 0.2542 0.2423] CrouchPlayer
  (`/Engine/EditorBlueprintResources/StandardMacros.IsValid` _interactableactor
    (:`Is Valid`
      (message `/Game/Blueprints/BPI/BPI_Interaction.TriggerWidget` _interactableactor)
      (bind _type (message `/Game/Blueprints/BPI/BPI_Interaction.InteractorType` _interactableactor))
      (switch `/Game/Blueprints/BPI/Enum_InteractorType` _type
        (:`NewEnumerator0`
          (set `self.isPicking` true))))))

(event `self.detectionZone.OnComponentBeginOverlap`
  (params (OverlappedComponent :type "PrimitiveComponent Object Reference") (OtherActor :type "Actor Object Reference") (OtherComp :type "PrimitiveComponent Object Reference") (OtherBodyIndex :type Integer) (bFromSweep :type Boolean) (SweepResult :type "HitResult Structure (by ref)"))
  ;[0 0.1501 0.3073] detectInteractor
  (if (`KismetSystemLibrary.DoesImplementInterface` OtherActor "/Game/Blueprints/BPI/BPI_Interaction.BPI_Interaction_C")
    (bind _output_get (set `self.interactableActor` OtherActor))
    (message `/Game/Blueprints/BPI/BPI_Interaction.ShowInteraction` _output_get true)))

(event `self.detectionZone.OnComponentEndOverlap`
  (params (OverlappedComponent :type "PrimitiveComponent Object Reference") (OtherActor :type "Actor Object Reference") (OtherComp :type "PrimitiveComponent Object Reference") (OtherBodyIndex :type Integer))
  ;[0 0.1501 0.3073] detectInteractor
  (if (`KismetSystemLibrary.DoesImplementInterface` OtherActor "/Game/Blueprints/BPI/BPI_Interaction.BPI_Interaction_C")
    (message `/Game/Blueprints/BPI/BPI_Interaction.ShowInteraction` OtherActor false)
    (set `self.interactableActor` null)))

(event `/Game/Blueprints/BPI/BPI_Player.LockpickWin`
  (bind _interactableactor (`self.interactableActor`))
  (bind _gameinstanceref (`self.gameInstanceRef`))
  (bind _score (`/Game/_Manager/inGame/GI_StealthGame.score` _gameinstanceref))
  (bind _playergameinterface (`/Game/_Manager/inGame/HUD_Player.playerGameInterface` (`self.As HUD Player`)))
  (bind _t_money (`/Game/Blueprints/UI/WB_GameInterface.T_Money` (`/Game/_Manager/inGame/HUD_Player.playerGameInterface` (`self.As HUD Player`))))
  (`/Engine/EditorBlueprintResources/StandardMacros.IsValid` _interactableactor
    (:`Is Valid`
      (bind (_score_2 _ismasterpiece) (message `/Game/Blueprints/BPI/BPI_Interaction.Interact` _interactableactor))
      (if (not (`self.masterPiece`))
        (set `self.masterPiece` _ismasterpiece))
      (set `self.isPicking` false)
      (set `self.score` _score)
      (bind _output_get (set `self.maxValue` (+ _score _score_2)))
      (`UserWidget.PlayAnimation` _playergameinterface (`/Game/Blueprints/UI/WB_GameInterface.Bounce` _playergameinterface) 0.0 1 "Forward" 1.0 false)
      (bind (_direction _alpha) (`Timeline|Timeline` :!via `PlayFromStart`)
        (:`Update`
          (set `/Game/_Manager/inGame/GI_StealthGame.score` (`KismetMathLibrary.FTrunc` (`KismetMathLibrary.Lerp` (`KismetMathLibrary.Conv_IntToDouble` (`self.score`)) (`KismetMathLibrary.Conv_IntToDouble` _output_get) _alpha)) _gameinstanceref)
          (`TextBlock.SetColorAndOpacity` _t_money (make `SlateColor` (`KismetMathLibrary.SelectColor` (struct :`R` 1.0 :`B` 0.007827 :`A` 1.0) (struct :`R` 1.0 :`G` 1.0 :`B` 1.0 :`A` 1.0) (< _score_2 0)))))
        (:`Finished`
          (set `/Game/_Manager/inGame/GI_StealthGame.scoreInLevel` (+ (`/Game/_Manager/inGame/GI_StealthGame.scoreInLevel` _gameinstanceref) _score_2) _gameinstanceref)
          (`TextBlock.SetColorAndOpacity` _t_money (make `SlateColor` (`KismetMathLibrary.SelectColor` (struct :`R` 1.0 :`B` 0.007827 :`A` 1.0) (struct :`R` 1.0 :`G` 1.0 :`B` 1.0 :`A` 1.0) (< (`/Game/_Manager/inGame/GI_StealthGame.score` _gameinstanceref) 0)))))))))

(event `/Game/Blueprints/BPI/BPI_Player.ResetHasMasterPiece`
  (set `self.masterPiece` false))

(event `/Game/Blueprints/BPI/BPI_Player.ResetGame`
  (bind _gameinstanceref (`self.gameInstanceRef`))
  (bind _outactors (`GameplayStatics.GetAllActorsOfClass` "/Game/Blueprints/GPE/ArtPieces/BP_ArtPiecesMASTER.BP_ArtPiecesMASTER_C"))
  (for _array_element _outactors
    (message `/Game/Blueprints/BPI/BPI_Interaction.Reset` _array_element))
  (`self.K2_SetActorLocation` (`self.spawnPos`))
  (set `/Game/_Manager/inGame/GI_StealthGame.score` (- (`/Game/_Manager/inGame/GI_StealthGame.score` _gameinstanceref) (`/Game/_Manager/inGame/GI_StealthGame.scoreInLevel` _gameinstanceref)) _gameinstanceref)
  (set `/Game/_Manager/inGame/GI_StealthGame.scoreInLevel` 0 _gameinstanceref)
  (bind _outactors_2 (`GameplayStatics.GetAllActorsOfClass` "/Game/Blueprints/Enemy/AI/AIC_Guard.AIC_Guard_C"))
  (for _array_element_2 _outactors_2
    (message `/Game/Blueprints/BPI/BPI_Enemy.ResetGame` _array_element_2))
  (`KismetSystemLibrary.Delay` 1.2)
  (message `/Game/Blueprints/BPI/BPI_HUD.ResetInputType` (`PlayerController.GetHUD` (`GameplayStatics.GetPlayerController` 0))))

(event `/Game/Blueprints/BPI/BPI_Player.NewSpawnPos`
  (params (newPos :type "Vector Structure"))
  (set `self.spawnPos` newPos))

(event `/Game/Blueprints/BPI/BPI_Player.LockPickLoose`
  (`self.MakeNoise` 0.4 null (`self.K2_GetActorLocation`) 0.0 "Hearing")
  (set `self.isPicking` false))

(fn `HasMasterPiece`
  (returns (masterPiece :type Boolean))
  (return (`self.masterPiece`)))

(fn `UserConstructionScript`
  (bind _dataassetref (`self.dataAssetRef`))
  (`parent.UserConstructionScript`)
  (`CameraComponent.SetFieldOfView` (`self.Camera`) (`/Game/DataAsset/BP_DataAsset.FOV` _dataassetref))
  (`SceneComponent.K2_SetRelativeLocationAndRotation` (`self.SpringArm`) (`/Game/DataAsset/BP_DataAsset.cameraOffset` _dataassetref) (`/Game/DataAsset/BP_DataAsset.cameraRotation` _dataassetref) false false))