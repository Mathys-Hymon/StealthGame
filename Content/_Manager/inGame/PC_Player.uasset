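; PC_Player is the player controller that turns Enhanced Input actions into commands for the player character.
; On BeginPlay it adds the IMC_Input mapping context to the local player subsystem.
; Move, Interact, Crouch and CancelAction events are forwarded to player character 0 as interface messages, so the controller holds no gameplay logic itself.
; Move also forwards the action value on cancel and completion.
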(event `self.ReceiveBeginPlay`
  (bind _returnvalue (subsystem `EnhancedInputLocalPlayerSubsystem`))
  ;[1 1 1] SetInputMapping
  (`/Engine/EditorBlueprintResources/StandardMacros.IsValid` _returnvalue
    (:`Is Valid`
      (message `EnhancedInputSubsystemInterface.AddMappingContext` _returnvalue "/Game/_Manager/Inputs/IMC_Input.IMC_Input" 0 (struct)))))

(event `EnhancedInput|/Game/_Manager/Inputs/actions/IA_Move`
  (params (ActionValue :type "Vector2D Structure") (ElapsedSeconds :type "Float (double-precision)") (TriggeredSeconds :type "Float (double-precision)") (InputAction :type "InputAction Object Reference" :default "/Game/_Manager/Inputs/actions/IA_Move.IA_Move"))
  ;[1 1 1] Move
  (:`Triggered`
    (message `/Game/Blueprints/BPI/BPI_Player.Move` (`GameplayStatics.GetPlayerCharacter` 0) ActionValue :!label _label))
  (:`Canceled`
    (goto _label))
  (:`Completed`
    (goto _label)))

(event `EnhancedInput|/Game/_Manager/Inputs/actions/IA_Interact`
  (params (ActionValue :type Boolean) (ElapsedSeconds :type "Float (double-precision)") (TriggeredSeconds :type "Float (double-precision)") (InputAction :type "InputAction Object Reference" :default "/Game/_Manager/Inputs/actions/IA_Interact.IA_Interact"))
  ;[1 1 1] Interact
  (:`Started`
    (message `/Game/Blueprints/BPI/BPI_Player.Interact` (`GameplayStatics.GetPlayerCharacter` 0))))

(event `EnhancedInput|/Game/_Manager/Inputs/actions/IA_Crouch`
  (params (ActionValue :type Boolean) (ElapsedSeconds :type "Float (double-precision)") (TriggeredSeconds :type "Float (double-precision)") (InputAction :type "InputAction Object Reference" :default "/Game/_Manager/Inputs/actions/IA_Crouch.IA_Crouch"))
  ;[1 1 1] Crouch
  (:`Started`
    (message `/Game/Blueprints/BPI/BPI_Player.CrouchPlayer` (`GameplayStatics.GetPlayerCharacter` 0))))

(event `EnhancedInput|/Game/_Manager/Inputs/actions/IA_CancelAction`
  (params (ActionValue :type Boolean) (ElapsedSeconds :type "Float (double-precision)") (TriggeredSeconds :type "Float (double-precision)") (InputAction :type "InputAction Object Reference" :default "/Game/_Manager/Inputs/actions/IA_CancelAction.IA_CancelAction"))
  ;[1 1 1] CancelAction
  (:`Started`
    (message `/Game/Blueprints/BPI/BPI_Player.CancelInteract` (`GameplayStatics.GetPlayerCharacter` 0))))

(fn `UserConstructionScript`)